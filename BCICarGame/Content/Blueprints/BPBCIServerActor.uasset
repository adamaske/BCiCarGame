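; Actor that runs a local OSC server on port 5700 to drive a Car from brain-computer interface (BCI) commands.
; Each bundle message's address and first float go to CheckCommand as command and strength.
; Matches against left, right, gas, brake and neutral commands set the Car's direction and strength.
; Space bar appears meant to toggle listening, but its inverted branch calls Listen again while already listening.
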(event Custom|BCI%20Bundle%20Get
  (params (Bundle :type OSC%20Bundle%20Structure%20%28by%20ref%29) (IPAddress :type String) (Port :type Integer))
  (bind _returnvalue (Class|OSCManager|GetMessagesfromBundle Bundle))
  (for _array_element _returnvalue
    (bind _returnvalue_2 (Class|OSCManager|GetOSCMessageAddress _array_element))
    (bind _returnvalue_3 (Class|OSCManager|GetOSCAddressFullPath _returnvalue_2))
    (bind _value (Class|OSCManager|GetFloat _array_element))
    (CallFunction|CheckCommand _returnvalue_3 _value)))

(event Custom|CheckCommand
  (params (Command :type String) (Strength :type Float%20%28single-precision%29))
  (Development|PrintString (Utilities|String|Append "Checking command " Command " with strength " (Utilities|String|ToString(Float) Strength)))
  (Utilities|FlowControl|Sequence
    (:then_0
      (if (Utilities|Enum|Equal(Enum) (Variables|Default|GetLeftCommand) Command)
        (Default|SetVelocityandStrength (Variables|Default|GetCar) "0.000000,-1.000000, 0" Strength)
        (Development|PrintString "Hello")))
    (:then_1
      (if (Utilities|Enum|Equal(Enum) (Variables|Default|GetRightCommand) Command)
        (Default|SetVelocityandStrength (Variables|Default|GetCar) "0.000000,1.000000, 0" Strength)))
    (:then_2
      (if (Utilities|Enum|Equal(Enum) (Variables|Default|GetGasCommand) Command)
        (Default|SetVelocityandStrength (Variables|Default|GetCar) "1.000000,0.000000, 0" Strength)))
    (:then_3
      (if (Utilities|Enum|Equal(Enum) (Variables|Default|GetBrakeCommand) Command)
        (Default|SetVelocityandStrength (Variables|Default|GetCar) "-1.000000,0.000000, 0" Strength)))
    (:then_4
      (if (Utilities|Enum|Equal(Enum) (Variables|Default|GetNeutralCommand) Command)
        (Default|SetVelocityandStrength (Variables|Default|GetCar) "0, 0, 0" Strength)))))

(event EventBeginPlay
  (Utilities|FlowControl|Sequence
    (:then_0
      (bind _returnvalue (Class|OSCManager|CreateOSCServer "127.0.0.1" 5700 false false "BCIServer" 0))
      (bind _output_get (Variables|Default|SetBCIServer _returnvalue))
      (Class|OSCServer|Listen _output_get)
      (Variables|Default|SetListening true)
      (Development|PrintString "IS Listeneing"))
    (:then_1
      (EventDispatchers|BindEventtoOnOscBundleReceived (Variables|Default|GetBCIServer) (delegate Custom|BCI%20Bundle%20Get)))))

(event Collision|EventActorBeginOverlap
  (params (OtherActor :type Actor%20Object%20Reference)))

(event EventTick
  (params (DeltaSeconds :type Float%20%28single-precision%29)))

(event Input|KeyboardEvents|SpaceBar
  (params (Key :type Key%20Structure :default "None"))
  (bind _bciserver (Variables|Default|GetBCIServer))
  (:Pressed
    (if (Variables|Default|GetListening)
      (Class|OSCServer|Listen _bciserver)
      (Variables|Default|SetListening true)
      (else
        (Class|OSCServer|Stop _bciserver)
        (Variables|Default|SetListening false)))))

(fn ConstructionScript)
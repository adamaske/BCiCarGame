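; Road manager actor that creates an endless scrolling road by recycling a line of BPRoadPiece actors.
; On BeginPlay it spawns the wanted number of pieces end to end along X.
; Each Tick slides them toward negative X and moves any piece a full length behind the origin to the back of the array.
; Each recycle then snaps all pieces to index-based positions to cancel floating-point drift, overriding the recycled piece's computed position.
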(event Custom|ResetRoadPiece
  (params (Piece :type BP%20Road%20Piece%20Object%20Reference))
  (bind _piecelength (Variables|Default|GetPieceLength))
  (bind _wantedpieces (Variables|Default|GetWantedPieces))
  (bind _piecesbehindcar (Variables|Default|GetPiecesBehindCar))
  (bind _piecelength_2 (Variables|Default|GetPieceLength))
  (bind _pieces (Variables|Default|GetPieces))
  (bind _returnvalue (/ _piecelength 2.0))
  (bind _returnvalue_2 (- _wantedpieces _piecesbehindcar))
  (bind _returnvalue_3 (* _piecelength_2 _returnvalue_2))
  (bind _returnvalue_4 (+ _returnvalue _returnvalue_3))
  ;[1 1 1] Move piece to back of line
  (Development|PrintString "Moved piece")
  (Transformation|SetActorLocation Piece (Math|Vector|MakeVector _returnvalue_4 0.0 0.0) false false)
  (Development|PrintString (Utilities|String|Append "Set piece X : " (Utilities|String|ToString(Float) _returnvalue_4)))
  (Utilities|Array|RemoveItem _pieces Piece)
  (Utilities|Array|Add _pieces Piece)
  (CallFunction|ResetAllPieces))

(event Custom|CheckPiecesPosition
  ;[1 1 1] Check if piece is behind player
  (for _array_element (Variables|Default|GetPieces)
    (if (<= (.X (Math|Vector|BreakVector (Transformation|GetActorLocation _array_element))) (- 0.0 (Variables|Default|GetPieceLength)))
      (CallFunction|ResetRoadPiece _array_element))))

(event Custom|MovePieces
  (params (deltaSeconds :type Float%20%28single-precision%29))
  ;[1 1 1] Moving peices
  (for _array_element (Variables|Default|GetPieces)
    (Transformation|AddActorLocalOffset _array_element (Math|Vector|MakeVector (- 0.0 (* (Variables|Default|GetPieceSpeed) deltaSeconds)) 0.0 0.0) false false)))

(event Custom|ResetAllPieces
  ;[1 1 1] Move All pieces to correct position,in case of floating point erro
  (for (_array_element _array_index) (Variables|Default|GetPieces)
    (Transformation|SetActorLocation _array_element (Math|Vector|MakeVector (* _array_index (Variables|Default|GetPieceLength)) 0.0 0.0) false false)))

(event EventBeginPlay
  ;[1 1 1] Spawn pieces
  (while (< (Variables|Default|GetPiecesAlive) (Variables|Default|GetWantedPieces))
    (bind _returnvalue (Game|SpawnActorfromClass "/Game/Blueprints/BPRoadPiece.BPRoadPiece_C" (Math|Transform|MakeTransform (Math|Vector|MakeVector (* (Variables|Default|GetPieceLength) (Variables|Default|GetPiecesAlive)) 0.0 0.0) "0, 0, 0" "1.000000,1,1") "Undefined" 0 0))
    (bind _returnvalue_2 (Utilities|Array|Add (Variables|Default|GetPieces) _returnvalue))
    (Development|PrintString (Utilities|String|Append "Spawned piece : " (Utilities|String|ToString(Integer) _returnvalue_2)))
    (Math|Float|IncrementFloat (Variables|Default|GetPiecesAlive))))

(event Collision|EventActorBeginOverlap
  (params (OtherActor :type Actor%20Object%20Reference)))

(event EventTick
  (params (DeltaSeconds :type Float%20%28single-precision%29))
  (CallFunction|CheckPiecesPosition)
  (CallFunction|MovePieces DeltaSeconds))

(fn ConstructionScript)
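; BPCarActor is a car actor that moves itself continuously through simple kinematic translation.
; Each Tick adds a local-space offset of Velocity scaled by delta time, CurrentSpeed and Strength, without sweeping for collision.
; SetVelocityAndStrength sets the Velocity and Strength values that drive this motion, while CurrentSpeed is only read here.
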(event EventBeginPlay)

(event Collision|EventActorBeginOverlap
  (params (OtherActor :type Actor%20Object%20Reference)))

(event EventTick
  (params (DeltaSeconds :type Float%20%28single-precision%29))
  (Transformation|AddActorLocalOffset self (* (Variables|Default|GetVelocity) (* DeltaSeconds (* (Variables|Default|GetCurrentSpeed) (Variables|Default|GetStrength)))) false false))

(fn ConstructionScript)

(fn SetVelocityandStrength
  (params (Vel :type Vector) (Strength :type Float%20%28single-precision%29))
  (Variables|Default|SetVelocity Vel)
  (Variables|Default|SetStrength Strength))